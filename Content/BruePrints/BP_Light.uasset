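; BP_Light is a checkpoint-style light that switches on when something overlaps its box and reports it to the game mode.
; The first overlap on the box collision passes a DoOnce, sets the Lightning flag and increments PassedLights on BP_MyGameMode, with no filter on the overlapping actor.
; Tick copies the Lightning flag to the point light's visibility every frame.
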(event `self.ReceiveTick`
  (params (DeltaSeconds :type "Float (single-precision)"))
  (`SceneComponent.SetVisibility` (`self.PointLight`) (`self.Lightning`) false))

(event `self.BoxClllision.OnComponentBeginOverlap`
  (params (OverlappedComponent :type "PrimitiveComponent Object Reference") (OtherActor :type "Actor Object Reference") (OtherComp :type "PrimitiveComponent Object Reference") (OtherBodyIndex :type Integer) (bFromSweep :type Boolean) (SweepResult :type "HitResult Structure (by ref)"))
  (`/Engine/EditorBlueprintResources/StandardMacros.DoOnce` false
    (:`Completed`
      (set `self.Lightning` true)
      (bind _asbp_my_game_mode (cast `/Game/BruePrints/BP_MyGameMode` (`GameplayStatics.GetGameMode`)))
      (set `/Game/BruePrints/BP_MyGameMode.PassedLights` (+ (`/Game/BruePrints/BP_MyGameMode.PassedLights` _asbp_my_game_mode) 1) _asbp_my_game_mode))))

(fn `UserConstructionScript`)